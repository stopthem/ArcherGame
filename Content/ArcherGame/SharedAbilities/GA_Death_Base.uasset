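; GA_Death_Base is a gameplay ability that plays an archer character's death when triggered by a gameplay event.
; After committing, it disables movement, stops the current montage and waits a tick.
; It picks a random directional death montage from a data asset using the yaw between effect causer and avatar.
; A montage-length delay, used because montage delegates fail without auto blend out, precedes FinishDeath on the HealthComponent and ending the ability.
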(event Ability|EventOnEndAbility
  (params (bWasCancelled :type Boolean)))

(event Ability|EventActivateAbilityFromEvent
  (params (EventData :type Gameplay%20Event%20Data%20Structure%20%28by%20ref%29))
  (bind _returnvalue (Class|ArcherGameplayAbility|GetArcherCharacterfromActorInfo))
  (bind _returnvalue_2 (Class|ArcherGameplayAbility|GetArcherCharacterfromActorInfo))
  (bind _healthcomponent (Variables|/Script/ArcherGame.ArcherCharacter|GetHealthComponent _returnvalue))
  (bind _returnvalue_3 (Ability|CommitAbility))
  (if _returnvalue_3
    (Pawn|Components|CharacterMovement|DisableMovement (Variables|/Script/Engine.Character|GetCharacterMovement _returnvalue_2))
    (Animation|StopAnimMontage _returnvalue_2 0)
    ;[0.01042 0.01042 0.01042] Currently playing montages will be stopped next tick
    (Utilities|FlowControl|DelayUntilNextTick)
    (bind _returnvalue_4 (Class|DirectionalAnimationDataAsset|GetRandomMontagefromDeltaAngle (Variables|Default|GetDirectionalAnimDataAsset) (.yaw (Math|Rotator|Delta(Rotator) (Transformation|GetActorRotation (Class|AbilitySystemBlueprintLibrary|EffectContextGetEffectCauser (.contexthandle EventData))) (Transformation|GetActorRotation (Ability|GetAvatarActorfromActorInfo))))))
    (|PlayMontageandWaitProxy "None" _returnvalue_4 1.0 "None" false 1.0 0.0
      (:then
        ;[0.01042 0.01042 0.01042] Waiting with delay because if montage's "Auto Blend Out" is false, the delegates does not work.
        (Utilities|FlowControl|Delay (Animation|GetPlayLength _returnvalue_4))
        ;[0.01042 0.01042 0.01042] Call Finish death if user is archer character and has a healthcomponent
        (Utilities|IsValid _returnvalue
          (:Is%20Valid
            (Utilities|IsValid _healthcomponent
              (:Is%20Valid
                (Class|ArcherHealthComponent|FinishDeath _healthcomponent)
                (Ability|EndAbility)))))))
    (else
      (Ability|CancelAbility))))
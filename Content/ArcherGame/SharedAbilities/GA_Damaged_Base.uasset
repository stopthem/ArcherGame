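; GA_Damaged_Base is a base gameplay ability that plays a directional hit-reaction montage when an ArcherGame character is damaged.
; On event activation it commits, then uses the yaw delta between instigator and target rotations to pick a montage from DirectionalAnimDataAsset.
; The montage plays slightly sped up only if no other is playing; otherwise the ability is never explicitly ended.
; Completion ends the ability, while interruption, cancellation or failed commit cancels it.
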(event Ability|EventOnEndAbility
  (params (bWasCancelled :type Boolean)))

(event Ability|EventActivateAbilityFromEvent
  (params (EventData :type Gameplay%20Event%20Data%20Structure%20%28by%20ref%29))
  (bind _returnvalue (Ability|CommitAbility))
  (if _returnvalue
    (if (not (Animation|Montage|MontageIsPlaying (Components|SkeletalMesh|GetAnimInstance (Variables|/Script/Engine.Character|GetMesh (Class|ArcherGameplayAbility|GetArcherCharacterfromActorInfo))) 0))
      ;[0.01042 0.01042 0.01042] Get to be played anim montage based on instigator and target delta rotation yaw
      (bind _returnvalue_2 (Class|DirectionalAnimationDataAsset|GetMontagefromDeltaAngle (Variables|Default|GetDirectionalAnimDataAsset) (.yaw (Math|Rotator|Delta(Rotator) (Transformation|GetActorRotation (.instigator EventData)) (Transformation|GetActorRotation (.target EventData))))))
      (|PlayMontageandWaitProxy "None" _returnvalue_2 1.25 "None" true 1.0 0.0
        (:OnCompleted
          (Ability|EndAbility))
        (:OnInterrupted
          (Ability|CancelAbility :!label _label))
        (:OnCancelled
          (goto _label))))
    (else
      (Ability|CancelAbility))))
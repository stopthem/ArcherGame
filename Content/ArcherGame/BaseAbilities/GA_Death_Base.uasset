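; GA_Death_Base is an event-activated Gameplay Ability that handles an archer character's death with a directional animation followed by ragdoll.
; After committing, it stops the current montage, waits a tick, then plays a random montage chosen from the instigator-to-target yaw delta via a directional anim data asset.
; After the montage's length, it simulates physics from the pelvis down, disables movement and capsule collision, then ends the ability.
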(event Ability|EventOnEndAbility
  (params (bWasCancelled :type Boolean)))

(event Ability|EventActivateAbilityFromEvent
  (params (EventData :type Gameplay%20Event%20Data%20Structure%20%28by%20ref%29))
  (bind _returnvalue (Class|ArcherGameplayAbility|GetArcherCharacterfromActorInfo))
  (bind _mesh (Variables|/Script/Engine.Character|GetMesh _returnvalue))
  (bind _returnvalue_2 (Ability|CommitAbility))
  (if _returnvalue_2
    (Animation|StopAnimMontage (Class|ArcherGameplayAbility|GetArcherCharacterfromActorInfo) 0)
    ;[1 1 1] Currently playing montages will be stopped next tick
    (Utilities|FlowControl|DelayUntilNextTick)
    (bind _returnvalue_3 (Class|DirectionalAnimationDataAsset|GetRandomMontagefromDeltaAngle (Variables|Default|GetDirectionalAnimDataAsset) (.yaw (Math|Rotator|Delta(Rotator) (Transformation|GetActorRotation (.instigator EventData)) (Transformation|GetActorRotation (.target EventData))))))
    (|PlayMontageandWaitProxy "None" _returnvalue_3 1.0 "None" false 1.0 0.0
      (:then
        (Utilities|FlowControl|Delay (- (Animation|GetPlayLength _returnvalue_3) 0.0))
        ;[1 1 1] Ragdoll TODO LYRA STYLE DEATH MATERIAL
        (Collision|SetCollisionEnabled _mesh "PhysicsOnly")
        (Class|SkeletalMeshComponent|SetAllBodiesBelowSimulatePhysics _mesh (Utilities|Name|MakeLiteralName "pelvis") true true)
        (Pawn|Components|CharacterMovement|DisableMovement (Variables|/Script/Engine.Character|GetCharacterMovement _returnvalue))
        (Collision|SetCollisionEnabled (Variables|/Script/Engine.Character|GetCapsuleComponent _returnvalue) "NoCollision")
        (Ability|EndAbility)))))
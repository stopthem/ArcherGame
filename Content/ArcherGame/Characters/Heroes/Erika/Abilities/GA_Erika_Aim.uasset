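; Gameplay ability for Erika's aim, which turns the player toward the mouse cursor while the input is held.
; On activation it flags the character as aiming, saves its movement rotation rate and applies an aiming rate.
; A tick task sets control rotation from the negated, normalized screen-center-to-cursor direction, flattened onto the XY plane.
; Input release ends the ability, clearing the flag and restoring the saved rate.
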(event Ability|EventActivateAbility
  (Utilities|FlowControl|Sequence
    (:then_0
      ;[1 1 1] Get ArcherPlayerCharacter
      (bind _asarcher_player_character (Utilities|Casting|CastToArcherPlayerCharacter (Ability|GetOwningActorfromActorInfo)))
      (bind _output_get (Variables|Default|SetArcherPlayerCharacter _asarcher_player_character))
      (Variables|/Script/ArcherGame.ArcherPlayerCharacter|SetIsAiming _output_get true))
    (:then_1
      ;[1 1 1] Calculate angle when player aiming for animations
      (|AbilityTaskonTick "None"
        (:OnTickTaskDelegate
          ;[1 1 1] Player look at mouse position
          (bind _returnvalue (Class|ScreenExBlueprintFunctionLibrary|GetScreenCentertoScreenPosDir (Math|Vector2D|MakeVector2D (.LocationX (Game|Player|GetMousePosition (Class|ArcherPlayerCharacter|GetPlayerController (Variables|Default|GetArcherPlayerCharacter)))) (.LocationY (Game|Player|GetMousePosition (Class|ArcherPlayerCharacter|GetPlayerController (Variables|Default|GetArcherPlayerCharacter))))) true true))
          (Pawn|SetControlRotation (Class|ArcherPlayerCharacter|GetPlayerController (Variables|Default|GetArcherPlayerCharacter)) (Math|Conversions|RotationFromXVector (Math|Vector|MakeVector (.x _returnvalue) (.y _returnvalue) 0.0))))))
    (:then_2
      (Ability|Tasks|WaitInputRelease false
        (:OnRelease
          (Ability|EndAbility))))
    (:then_3
      (Variables|Default|SetOldRotationRate (Variables|/Script/Engine.CharacterMovementComponent|GetRotationRate (Variables|/Script/Engine.Character|GetCharacterMovement (Variables|Default|GetArcherPlayerCharacter))))
      (Variables|/Script/Engine.CharacterMovementComponent|SetRotationRate (Variables|/Script/Engine.Character|GetCharacterMovement (Variables|Default|GetArcherPlayerCharacter)) (Variables|Default|GetAimingRotationRate)))))

(event Ability|EventOnEndAbility
  (params (bWasCancelled :type Boolean))
  (bind _archerplayercharacter (Variables|Default|GetArcherPlayerCharacter))
  (Utilities|FlowControl|Sequence
    (:then_0
      (Variables|/Script/ArcherGame.ArcherPlayerCharacter|SetIsAiming _archerplayercharacter false))
    (:then_1
      (Variables|/Script/Engine.CharacterMovementComponent|SetRotationRate (Variables|/Script/Engine.Character|GetCharacterMovement _archerplayercharacter) (Variables|Default|GetOldRotationRate)))))
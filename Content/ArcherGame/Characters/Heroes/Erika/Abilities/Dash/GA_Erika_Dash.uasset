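; Erika's dash Gameplay Ability, which launches the character along movement input or facing with a matching directional montage.
; On a locally controlled avatar it picks the montage by input-to-facing yaw, then commits.
; With authority, it turns the avatar unless aiming, plays the rate-scaled montage and applies constant-force root motion.
; When the force finishes, it plays a stopping montage and delays ending to block immediate cancelling into other actions.
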(event Ability|EventActivateAbility
  (bind _returnvalue (Ability|GetAvatarActorfromActorInfo))
  (bind (_facing _last_movement_input _positive) (|GetDirection_2))
  (Utilities|FlowControl|Sequence
    (:then_0
      (Pawn|IsLocallyControlled
        (:True
          ;[1 1 1] Calculate dash direction and select appropriate animation
          (bind _directionalmontage (CallFunction|SelectDirectionalMontage _facing _last_movement_input))
          (Variables|Dash|Montage|SetMontage _directionalmontage)
          (bind _output_get (Variables|Dash|SetDirection (select _positive _last_movement_input _facing)))
          ;[1 1 1] If we have a non-zero dash, commit the ability
          (if (Math|Vector|VectorIsNearlyZero _output_get)
            (Ability|CancelAbility :!label _label)
            (else
              (bind _returnvalue_2 (Ability|CommitAbility))
              (if _returnvalue_2
                (Ability|HasAuthority
                  (:True
                    (Utilities|FlowControl|Sequence
                      (:then_0
                        (bind _playrate (CallFunction|CalculateAnimPlayRate)))
                      (:then_1
                        (if (not (GameplayTags|HasTag (GameplayTags|GetOwnedGameplayTags (Ability|GetAbilitySystemComponentfromActorInfo) :!class /Script/GameplayTags.GameplayTagAssetInterface) "(TagName=\"Event.Aiming\")" true))
                          ;[1 1 1] Rotate towards dashing direction
                          (Transformation|SetActorRotation _returnvalue (Math|Conversions|RotationFromXVector _output_get))))
                      (:then_2
                        (|PlayMontageandWaitProxy "None" (Variables|Dash|Montage|GetMontage) _playrate "None" false 1.0 0.0
                          (:then
                            ;[1 1 1] Use values to apply root motion to pawn
                            (Ability|Tasks|ApplyRootMotionConstantForce "None" (Variables|Dash|GetDirection) (Variables|Dash|GetStrength) (Variables|Dash|GetRootMotionDuration) true 0 "ClampVelocity" (Transformation|GetVelocity _returnvalue) 1e+03
                              (:OnFinish
                                (Utilities|FlowControl|Sequence
                                  (:then_0
                                    ;[1 1 1] Delay end of ability so you can't immediately cancel into another action
                                    (Utilities|FlowControl|Delay (- (Variables|Dash|GetAbilityDuration) (Variables|Dash|GetRootMotionDuration)))
                                    (Ability|EndAbility))
                                  (:then_1
                                    ;[1 1 1] Play stopping montage if there is no montage playing
                                    (Animation|Montage|PlayMontage (Variables|/Script/Engine.Character|GetMesh (Variables|Default|GetArcherPlayerCharacter)) (Variables|Dash|Montage|GetStoppingMontage)))))))
                          (:OnInterrupted
                            (Ability|EndAbility :!label _label_2))
                          (:OnCancelled
                            (goto _label_2)))))))
                (else
                  (goto _label))))))))
    (:then_1
      (bind _asarcher_player_character (Utilities|Casting|CastToArcherPlayerCharacter (Ability|GetOwningActorfromActorInfo)))
      (Variables|Default|SetArcherPlayerCharacter _asarcher_player_character))))

(fn SelectDirectionalMontage
  (params (Facing%20Direction :type Vector) (Movement%20Direction :type Vector))
  (bind _returnvalue (Math|Conversions|RotationFromXVector Facing%20Direction))
  (bind _returnvalue_2 (Math|Conversions|RotationFromXVector Movement%20Direction))
  (bind _returnvalue_3 (Math|Rotator|Delta(Rotator) _returnvalue_2 _returnvalue))
  (bind _returnvalue_4 (Math|Float|Absolute(Float) (.yaw _returnvalue_3)))
  (if (< _returnvalue_4 45.0)
    (LocalVariables|SetMontageToPick (Variables|Dash|Montage|GetDash_Fwd%20Montage))
    (elif (> _returnvalue_4 135.0)
      (LocalVariables|SetMontageToPick (Variables|Dash|Montage|GetDash_Bwd%20Montage))
      (elif (< (.yaw _returnvalue_3) 0.0)
        (LocalVariables|SetMontageToPick (Variables|Dash|Montage|GetDash_Left%20Montage))
        (else
          (LocalVariables|SetMontageToPick (Variables|Dash|Montage|GetDash_Right%20Montage))))))
  (return (LocalVariables|GetMontageToPick)))

(fn CalculateAnimPlayRate
  (return (/ (/ (Animation|GetPlayLength (Variables|Dash|Montage|GetMontage)) (Variables|Dash|GetRootMotionDuration)) 2.0)))
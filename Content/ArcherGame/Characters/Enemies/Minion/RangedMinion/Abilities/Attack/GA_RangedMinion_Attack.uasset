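; Gameplay ability for the ranged minion's attack, which fires a projectile at the AI's blackboard TargetActor.
; It plays a random attack montage rate-fitted to the remaining cooldown, spawning the projectile and muzzle VFX on the GameplayEvent.Attack event.
; A tick task turns the minion toward the target and cancels if the target is invalid or out of range.
; Character movement uses controller rotation until the ability ends.
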(event Ability|EventActivateAbility
  (bind _returnvalue (Class|ArcherGameplayAbility|GetArcherCharacterfromActorInfo))
  (bind _returnvalue_2 (Class|ArcherGameplayAbility|GetArcherCharacterfromActorInfo))
  (bind _attackingmontages (Variables|Default|GetAttackingMontages))
  (bind _outitem (Utilities|Array|Random _attackingmontages))
  (|CallParentFunction)
  (bind _returnvalue_3 (Ability|CommitAbility))
  (if _returnvalue_3
    (CallFunction|CharacterMovementUseControlRotation true)
    (Utilities|FlowControl|Sequence
      (:then_0
        ;[0.01042 0.01042 0.01042] Get target actor from blackboard
        (bind _asactor (Utilities|Casting|CastToActor (AI|Components|Blackboard|GetValueasObject (Variables|/Script/AIModule.AIController|GetBlackboard (Variables|Default|GetArcherEnemyAIController)) (Utilities|Name|MakeLiteralName "TargetActor"))))
        (Variables|Default|SetTargetActor _asactor))
      (:then_1
        ;[0.01042 0.01042 0.01042] Get ranged minion bp
        (bind _asbp_ranged_minion (Utilities|Casting|CastToBP_RangedMinion (Class|ArcherGameplayAbility|GetArcherCharacterfromActorInfo)))
        (Variables|Default|SetRangedMinionBP _asbp_ranged_minion))
      (:then_2
        ;[0.01042 0.01042 0.01042] Play montage and wait for anim notify gameplay event
        (|PlayMontageandWaitforEvent "None" _outitem "(GameplayTags=((TagName=\"GameplayEvent.Attack\")))" (Class|AnimBlueprintFunctionLibrary|GetPlayRatefromTime _outitem (Class|GameplayAbility|GetCooldownTimeRemaining)) "None" true 1.0
          (:OnCompleted
            (Ability|EndAbility))
          (:OnInterrupted
            (Ability|CancelAbility :!label _label))
          (:OnCancelled
            (goto _label))
          (:EventReceived
            ;[0.01042 0.01042 0.01042] Spawn projectile and fire towards target
            (Components|Activation|Activate (Variables|/Game/ArcherGame/Characters/Enemies/Minion/RangedMinion/BP_RangedMinion.BP_RangedMinion_C|GetMuzzleVFX (Variables|Default|GetRangedMinionBP)) true)
            (bind _returnvalue_4 (Game|SpawnActorfromClass "/Game/ArcherGame/Characters/Enemies/Minion/RangedMinion/Shooting/BP_RangedMinion_Projectile.BP_RangedMinion_Projectile_C" (Math|Transform|MakeTransform (Transformation|GetSocketLocation (Variables|/Script/Engine.Character|GetMesh _returnvalue) "Muzzle_Front") (Transformation|GetActorRotation _returnvalue) "1.000000,1.000000,1.000000") "AlwaysSpawn" 0 0))
            (Class|ArcherProjectileBase|Shoot _returnvalue_4 (Class|ArcherGameplayAbility|GetArcherCharacterfromActorInfo)))))
      (:then_3
        (bind _deltatime (|AbilityTaskonTick "None")
          (:OnTickTaskDelegate
            (Utilities|FlowControl|Sequence
              (:then_0
                ;[0.01042 0.01042 0.01042] Cancel ability if there is no target actor
                (if (not (Utilities|IsValid (Variables|Default|GetTargetActor)))
                  (Ability|CancelAbility)))
              (:then_1
                ;[0.01042 0.01042 0.01042] Rotate towards target untill firing
                (Transformation|SetActorRotation _returnvalue_2 (Class|KismetMathLibrary|RInterptoConstant (Transformation|GetActorRotation _returnvalue_2) (Math|Rotator|FindLookatRotation (Transformation|GetActorLocation _returnvalue_2) (Transformation|GetActorLocation (Variables|Default|GetTargetActor))) _deltatime 75.0) true))
              (:then_2
                ;[0.01042 0.01042 0.01042] Cancel ability if target is not in range
                (if (not (<= (Math|Vector|Distance2D(Vector) (Transformation|GetActorLocation (Variables|Default|GetTargetActor)) (Transformation|GetActorLocation (Class|ArcherGameplayAbility|GetArcherCharacterfromActorInfo))) (Variables|/Game/ArcherGame/Characters/Enemies/Minion/Shared/AI/AI_Minion.AI_Minion_C|GetDamageRange (Variables|Default|GetAIMinionBP))))
                  (Ability|CancelAbility))))))))
    (else
      (Ability|CancelAbility))))

(event Ability|EventOnEndAbility
  (params (bWasCancelled :type Boolean))
  (CallFunction|CharacterMovementUseControlRotation false))

(fn CharacterMovementUseControlRotation
  (params (UseControlRotation :type Boolean))
  (bind _returnvalue (Class|ArcherGameplayAbility|GetArcherCharacterfromActorInfo))
  (bind _charactermovement (Variables|/Script/Engine.Character|GetCharacterMovement _returnvalue))
  (Variables|/Script/Engine.CharacterMovementComponent|SetbOrientRotationToMovement _charactermovement (not UseControlRotation))
  (Variables|/Script/Engine.CharacterMovementComponent|SetbUseControllerDesiredRotation _charactermovement UseControlRotation))
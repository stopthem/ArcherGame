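; BP_Minion_Base is the base Blueprint for minion enemies, responsible for setting up their health bar.
; On BeginPlay, HandleHealthBar casts the widget component's user widget to WBP_Enemy_HealthBar, caches it and passes it the minion's HealthComponent.
; It then attaches the widget component to the mesh's HealthBar socket, snapping location while keeping relative rotation and scale.
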(event EventBeginPlay
  (CallFunction|HandleHealthBar))

(event Collision|EventActorBeginOverlap
  (params (OtherActor :type Actor%20Object%20Reference)))

(event EventTick
  (params (DeltaSeconds :type Float%20%28single-precision%29)))

(fn ConstructionScript)

(fn HandleHealthBar
  ;[0.01042 0.01042 0.01042] Set health bar bp
  (bind _aswbp_enemy_health_bar (Utilities|Casting|CastToWBP_Enemy_HealthBar (UserInterface|GetUserWidgetObject (Variables|HealthBar|GetHealthBarWidget))))
  (bind _output_get (Variables|HealthBar|SetHealthBarBP _aswbp_enemy_health_bar))
  (Variables|/Game/ArcherGame/Characters/Enemies/Widgets/WBP_Enemy_HealthBar.WBP_Enemy_HealthBar_C|SetHealthComponent _output_get (Variables|Default|GetHealthComponent))
  ;[0.01042 0.01042 0.01042] Attach to Health Bar Socket
  (Transformation|AttachComponentToComponent (Variables|HealthBar|GetHealthBarWidget) (Variables|Character|GetMesh) "HealthBar" "SnapToTarget" "KeepRelative" "KeepRelative" true))
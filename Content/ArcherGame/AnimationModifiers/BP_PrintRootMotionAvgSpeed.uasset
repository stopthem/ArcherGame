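; Animation modifier that logs the average root motion speed of an animation sequence when applied.
; It measures the straight-line distance between the root bone's location at the default frame and at the frame-count index, then divides it by the sequence length.
; The result prints to the log only, and the animation is left unmodified.
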(event EventOnApply
  (params (AnimationSequence :type Anim%20Sequence%20Object%20Reference))
  (bind _rootbonename (Variables|Default|GetRootBoneName))
  (bind _returnvalue (Utilities|String|StringToName _rootbonename))
  (Development|PrintString 0 (Utilities|String|Append "Average Speed" (Utilities|String|ToString(Float) (/ (Math|Vector|VectorLength (- (.location (Class|AnimationBlueprintLibrary|GetBonePoseforFrame AnimationSequence _returnvalue 0 false)) (.location (Class|AnimationBlueprintLibrary|GetBonePoseforFrame AnimationSequence _returnvalue (Class|AnimationBlueprintLibrary|GetNumFrames AnimationSequence) false)))) (Class|AnimationBlueprintLibrary|GetSequenceLength AnimationSequence)))) false))
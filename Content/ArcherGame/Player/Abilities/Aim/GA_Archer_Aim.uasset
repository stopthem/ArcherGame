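; Gameplay ability for the archer's aim, which charges shot power while the aim input is held.
; Each tick it raises power, turns control yaw toward the cursor, snapping to actors with ability systems, and updates the power bar.
; Until the timed knocking montage completes, the bar's widget length follows a predicted arrow path using a pooled projectile's speed.
; Release passes power to GA_Archer_Shoot, activates it and ends aiming, restoring rotation rate.
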(event Ability|EventActivateAbility
  (bind _returnvalue (Class|ArcherGameplayAbility|GetArcherPlayerCharacterfromActorInfo))
  (bind _charactermovement (Variables|/Script/Engine.Character|GetCharacterMovement _returnvalue))
  (bind _returnvalue_2 (Ability|CommitAbility))
  (if _returnvalue_2
    (Utilities|FlowControl|Sequence
      (:then_0
        (CallFunction|GetAbilitySystemNShootAbility))
      (:then_1
        (CallFunction|GetPlayerRelatedVariables))
      (:then_2
        (CallFunction|GetProjectileforWidgetSizeCalculations))
      (:then_3
        ;[0.01042 0.01042 0.01042] If player releases aim button, try playing shooting ability and end ability
        (Ability|Tasks|WaitInputRelease false
          (:OnRelease
            (Variables|/Game/ArcherGame/Player/Abilities/Shooting/GA_Archer_Shoot.GA_Archer_Shoot_C|SetShootingPower (Variables|Ability|Shoot|GetShootAbility) (Variables|ShootingPower|GetShootingPower))
            (Class|AbilitySystemComponent|TryActivateAbility (Variables|Ability|GetArcherAbilitySystemComponent) (Variables|Ability|Shoot|GetShootGameplayAbilitySpecHandle) true)
            (Ability|EndAbility))))
      (:then_4
        (CallFunction|SetShootingPowerIncreaseSpeed))
      (:then_5
        ;[0.01042 0.01042 0.01042] Play Knocking Anim
        (|PlayMontageandWaitProxy "None" (Variables|Ability|Shoot|GetArrowKnockingMontage) (Class|AnimBlueprintFunctionLibrary|GetPlayRatefromTime (Variables|Ability|Shoot|GetArrowKnockingMontage) (Variables|ShootingPower|GetFullShootingPowerTime)) "None" true 1.0 0.0
          (:OnCompleted
            (Variables|Default|SetShouldUpdateShootingPowerWidgetSize false)
            (Default|OnShootPowerFull (Variables|ShootingPower|GetShootPowerProgressBar)))))
      (:then_6
        (bind _deltatime (|AbilityTaskonTick "None")
          (:OnTickTaskDelegate
            (Utilities|FlowControl|Sequence
              (:then_0
                (CallFunction|UpdateShootingPowerWidgetSize))
              (:then_1
                (CallFunction|SetControlRotation))
              (:then_2
                ;[0.01042 0.01042 0.01042] increase power
                (bind _output_get (Variables|ShootingPower|SetShootingPower (Math|Float|Clamp(Float) (+ (Variables|ShootingPower|GetShootingPower) (* _deltatime (Variables|ShootingPower|GetShootingPowerIncreaseSpeed))))))
                ;[0.01042 0.01042 0.01042] Set shooting power widget percent
                (Variables|/Game/ArcherGame/Player/Abilities/Shooting/Assets/Widgets/WBP_ShootPowerProgressBar.WBP_ShootPowerProgressBar_C|SetPercent (Variables|ShootingPower|GetShootPowerProgressBar) _output_get))))))
      (:then_7
        ;[0.01042 0.01042 0.01042] Set character movement rotation rate to something faster and save the old one
        (Variables|RotationRate|SetOldRotationRate (Variables|/Script/Engine.CharacterMovementComponent|GetRotationRate _charactermovement))
        (Variables|/Script/Engine.CharacterMovementComponent|SetRotationRate _charactermovement (Variables|RotationRate|GetAimingRotationRate))))
    (else
      (Ability|CancelAbility))))

(event Ability|EventOnEndAbility
  (params (bWasCancelled :type Boolean))
  ;[0.01042 0.01042 0.01042] Set old rotation rate back to character movement
  (Variables|/Script/Engine.CharacterMovementComponent|SetRotationRate (Variables|/Script/Engine.Character|GetCharacterMovement (Class|ArcherGameplayAbility|GetArcherPlayerCharacterfromActorInfo)) (Variables|RotationRate|GetOldRotationRate))
  ;[0.01042 0.01042 0.01042] Hide shooting power widget
  (Widget|SetVisibility (Variables|ShootingPower|GetShootPowerProgressBar) "Hidden"))

(fn SetShootingPowerWidgetSize
  (bind _returnvalue (Class|ArcherGameplayAbility|GetArcherPlayerCharacterfromActorInfo))
  (bind _archerplayerbp (Variables|Default|GetArcherPlayerBP))
  (bind _shootingpowerwidget (Variables|/Game/ArcherGame/Player/BP_Player.BP_Player_C|GetShootingPowerWidget _archerplayerbp))
  (bind _outhit (Class|GameplayStatics|BlueprintPredictProjectilePathbyTraceChannel (Transformation|GetSocketLocation (Variables|/Script/Engine.Character|GetMesh _returnvalue) "arrow_anchor") (* (Variables|/Script/Engine.ProjectileMovementComponent|GetMaxSpeed (Variables|/Script/ArcherGame.ArcherProjectileBase|GetProjectileMovementComponent (Variables|Default|GetArrowProjectile))) (Transformation|GetActorForwardVector _returnvalue)) true 0.0 "ECC_GameTraceChannel6" false (Utilities|Array|MakeArray _returnvalue) "None" 1.0 3e+01 1.0))
  (Class|WidgetComponent|SetDrawSize _shootingpowerwidget (Math|Vector2D|MakeVector2D (Math|Vector|Distance(Vector) (.location _outhit) (Transformation|GetActorLocation _returnvalue)) (.y (Class|WidgetComponent|GetDrawSize _shootingpowerwidget)))))

(fn GetAbilitySystemNShootAbility
  (bind _returnvalue (Class|ArcherGameplayAbility|GetArcherPlayerCharacterfromActorInfo))
  (bind _returnvalue_2 (Class|ArcherCharacter|GetArcherAbilitySystemComponent _returnvalue))
  (Variables|Ability|SetArcherAbilitySystemComponent _returnvalue_2)
  (bind _out_gameplayabilityspechandle (Class|ArcherAbilitySystemComponent|FindAbilitySpecHandlefromTag _returnvalue_2 "(TagName=\"Ability.Shooting\")"))
  (bind _output_get (Variables|Ability|Shoot|SetShootGameplayAbilitySpecHandle _out_gameplayabilityspechandle))
  (bind _asga_archer_shoot (Utilities|Casting|CastToGA_Archer_Shoot (.ReturnValue (Ability|GameplayAbility|GetGameplayAbilityfromSpecHandle (Variables|Ability|GetArcherAbilitySystemComponent) _output_get))))
  (Variables|Ability|Shoot|SetShootAbility _asga_archer_shoot))

(fn GetPlayerRelatedVariables
  ;[0.01042 0.01042 0.01042] Get player bp and shooting power widget
  (bind _asbp_player (Utilities|Casting|CastToBP_Player (Class|ArcherGameplayAbility|GetArcherPlayerCharacterfromActorInfo)))
  (bind _output_get (Variables|Default|SetArcherPlayerBP _asbp_player))
  (bind _output_get_2 (Variables|ShootingPower|SetShootPowerProgressBar (Variables|/Game/ArcherGame/Player/BP_Player.BP_Player_C|GetShootPowerProgressBar _output_get)))
  (Widget|SetVisibility _output_get_2 "Visible"))

(fn GetProjectileforWidgetSizeCalculations
  ;[0.01042 0.01042 0.01042] Get arrow projectile for shooting power widget size calculations
  (bind _returnvalue (Class|PoolerSubsystem|GetPoolerfromGameplayTag (Subsystems|GetPoolerSubsystem) "(TagName=\"Pool.Arrow\")"))
  (bind _asarrow_projectile (Utilities|Casting|CastToArrowProjectile (Components|GetOwner (Utilities|Array|Get(acopy) (Variables|/Script/Pooling.Pooler|GetPooledActors _returnvalue)))))
  (Variables|Default|SetArrowProjectile _asarrow_projectile))

(fn SetShootingPowerIncreaseSpeed
  ;[0.01042 0.01042 0.01042] Set power increase speed
  (Variables|ShootingPower|SetShootingPowerIncreaseSpeed (/ 1.0 (Variables|ShootingPower|GetFullShootingPowerTime)))
  (Variables|ShootingPower|SetShootingPower (Variables|ShootingPower|GetMinShootingPower)))

(fn UpdateShootingPowerWidgetSize
  ;[0.01042 0.01042 0.01042] Update shooting power widget size if knocking animation is not complete
  (if (Variables|Default|GetShouldUpdateShootingPowerWidgetSize)
    (CallFunction|SetShootingPowerWidgetSize)))

(fn UpdateShootingPowerWidgetVisibility
  ;[0.01042 0.01042 0.01042] Handle shooting power widget visibility
  (bind _output_get (Variables|Ability|Shoot|SetCanShoot (not (GameplayTags|HasMatchingGameplayTag (Variables|Ability|GetArcherAbilitySystemComponent) "(TagName=\"Ability.Shooting.Cooldown\")"))))
  (Widget|SetVisibility (Variables|ShootingPower|GetShootPowerProgressBar) (select _output_get "Visible" "Hidden")))

(fn SetControlRotation
  (bind _returnvalue (Class|ArcherGameplayAbility|GetArcherPlayerCharacterfromActorInfo))
  (bind _returnvalue_2 (Class|ArcherPlayerCharacter|GetPlayerController _returnvalue))
  (bind _hitresult (Game|Player|GetHitResultUnderCursorbyChannel _returnvalue_2 "TraceTypeQuery3" true))
  (bind (_bblockinghit _binitialoverlap _time _distance _location _impactpoint _normal _impactnormal _physmat _hitactor) (Collision|BreakHitResult _hitresult))
  ;[0.01042 0.01042 0.01042] Set actor control rotation
  (if _bblockinghit
    (Pawn|SetControlRotation _returnvalue_2 (Math|Rotator|MakeRotator 0.0 0.0 (.yaw (Math|Rotator|FindLookatRotation (Class|PlayerController|GetFocalLocation _returnvalue_2) (select (Utilities|IsValid (Ability|GetAbilitySystemComponent _hitactor)) (Transformation|GetActorLocation _hitactor) _location)))))))
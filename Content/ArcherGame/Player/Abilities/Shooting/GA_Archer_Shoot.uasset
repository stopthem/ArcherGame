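; Gameplay ability that fires the archer's arrow once the ability commits.
; It plays the shoot montage at a rate derived from the remaining cooldown, ending when the montage completes or is interrupted or cancelled.
; Alongside, it takes an arrow from the tag-identified pool, scales initial speed by ShootingPower, then launches it from the mesh's arrow_anchor socket along control rotation.
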(event Ability|EventActivateAbility
  (bind _returnvalue (Ability|CommitAbility))
  (if _returnvalue
    (Utilities|FlowControl|Sequence
      (:then_0
        ;[1 1 1] Play montage and end ability when it finished
        (|PlayMontageandWaitProxy "None" (Variables|Default|GetShootMontage) (Class|AnimBlueprintFunctionLibrary|GetPlayRatefromTime (Variables|Default|GetShootMontage) (Class|GameplayAbility|GetCooldownTimeRemaining)) "None" true 1.0 0.0
          (:OnCompleted
            _)
          (:OnInterrupted
            _)
          (:OnCancelled
            _))
        (Ability|EndAbility))
      (:then_1
        ;[1 1 1] Spawn and shoot arrow
        (bind _returnvalue_2 (Class|PoolerBlueprintFunctionLibrary|GetPoolerbyGameplayTag "(TagName=\"Pool.Arrow\")"))
        (bind _returnvalue_3 (Class|Pooler|GetPooledObj _returnvalue_2))
        (bind _output_get (Variables|Default|SetArrow _returnvalue_3))
        (Utilities|FlowControl|Sequence
          (:then_0
            ;[1 1 1] Set initial speed of the projectile movement 0 to already set value and alpha of calculated aim ability power
            (bind _asarrow_projectile (Utilities|Casting|CastToArrowProjectile _output_get))
            (bind _output_get_2 (Variables|Default|SetArrowProjectile _asarrow_projectile))
            (Variables|/Script/Engine.ProjectileMovementComponent|SetInitialSpeed (Variables|/Script/ArcherGame.ArcherProjectileBase|GetProjectileMovementComponent _output_get_2) (Math|Float|Lerp 0.0 (Variables|/Script/Engine.ProjectileMovementComponent|GetMaxSpeed (Variables|/Script/ArcherGame.ArcherProjectileBase|GetProjectileMovementComponent _output_get_2)) (Variables|Default|GetShootingPower))))
          (:then_1
            (Transformation|SetActorLocationAndRotation (Variables|Default|GetArrow) (.location (Transformation|GetSocketTransform (Variables|/Script/Engine.Character|GetMesh (Class|ArcherGameplayAbility|GetArcherPlayerCharacterfromActorInfo)) "arrow_anchor" "RTS_World")) (Pawn|GetControlRotation (Class|ArcherGameplayAbility|GetArcherPlayerCharacterfromActorInfo) :!class /Script/Engine.Pawn) false true)
            (Transformation|SetActorScale3D (Variables|Default|GetArrow) "0.750000,0.750000,0.500000")
            (Class|ArcherProjectileBase|Shoot (Variables|Default|GetArrowProjectile))))))))

(event Ability|EventOnEndAbility
  (params (bWasCancelled :type Boolean)))
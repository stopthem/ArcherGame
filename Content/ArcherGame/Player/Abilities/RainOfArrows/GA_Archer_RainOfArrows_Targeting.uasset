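; Targeting ability for the archer's Rain of Arrows, letting the player place the strike area under the cursor.
; It plays a targeting montage, spawns a radius-scaled target actor, then each tick moves it to the cursor hit and yaws the player toward it, favoring ability-system actors.
; When the Fire ability activates it hands over target and radius and ends; losing the Event.RainOfArrows tag cancels and destroys the target.
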(event Ability|EventActivateAbility
  (bind _returnvalue (Ability|CommitAbility))
  (if _returnvalue
    (Utilities|FlowControl|Sequence
      (:then_0
        ;[0.01042 0.01042 0.01042] Play targeting montage and spawn target actor
        (|PlayMontageandWaitProxy "None" (Variables|Default|GetTargetingAnimMontage) 1.0 "None" true 1.0 0.0
          (:then
            (bind _returnvalue_2 (Game|SpawnActorfromClass "/Game/ArcherGame/Player/Abilities/RainOfArrows/Assets/BP_RainOfArrows_Target.BP_RainOfArrows_Target_C" (Math|Transform|MakeTransform "0, 0, 0" "0, 0, 0" (Math|Conversions|ToVector(Float) (/ (Variables|Default|GetRadius) 1e+02))) "AlwaysSpawn" 0 0))
            (Variables|Default|SetRainOfArrowsTarget _returnvalue_2))))
      (:then_1
        ;[0.01042 0.01042 0.01042] Wait for GA_Archer_RainOfArrows_Fire to activate and set its values then end this ability
        (bind _activatedability (|WaitforAbilityActivate :WithTag "(TagName=\"Ability.RainOfArrows.Fire\")")
          (:OnActivate
            (GameplayTasks|EndTask (stale _asynctaskproxy))
            (Utilities|FlowControl|Sequence
              (:then_0
                (bind _asga_archer_rain_of_arrows_fire (Utilities|Casting|CastToGA_Archer_RainOfArrows_Fire _activatedability))
                (Variables|/Game/ArcherGame/Player/Abilities/RainOfArrows/GA_Archer_RainOfArrows_Fire.GA_Archer_RainOfArrows_Fire_C|SetRainOfArrowsTarget _asga_archer_rain_of_arrows_fire (Variables|Default|GetRainOfArrowsTarget))
                (Variables|/Game/ArcherGame/Player/Abilities/RainOfArrows/GA_Archer_RainOfArrows_Fire.GA_Archer_RainOfArrows_Fire_C|SetRadius _asga_archer_rain_of_arrows_fire (Variables|Default|GetRadius)))
              (:then_1
                (Ability|EndAbility))))))
      (:then_2
        (bind _asynctaskproxy (Ability|Tasks|WaitGameplayTagRemove "(TagName=\"Event.RainOfArrows\")" 0)
          (:Removed
            (Ability|CancelAbility))))
      (:then_3
        (|AbilityTaskonTick "None"
          (:OnTickTaskDelegate
            ;[0.01042 0.01042 0.01042] Set rain of arrow target and actor control rotation
            (Variables|Default|SetPlayerController (Class|ArcherPlayerCharacter|GetPlayerController (Class|ArcherGameplayAbility|GetArcherPlayerCharacterfromActorInfo)))
            (if (.bBlockingHit (Collision|BreakHitResult (.HitResult (Game|Player|GetHitResultUnderCursorbyChannel (Variables|Default|GetPlayerController) "TraceTypeQuery4" true))))
              (Utilities|FlowControl|Sequence
                (:then_0
                  (Pawn|SetControlRotation (Variables|Default|GetPlayerController) (Math|Rotator|MakeRotator 0.0 0.0 (.yaw (Math|Rotator|FindLookatRotation (Class|PlayerController|GetFocalLocation (Variables|Default|GetPlayerController)) (select (Utilities|IsValid (Ability|GetAbilitySystemComponent (.HitActor (Collision|BreakHitResult (.HitResult (Game|Player|GetHitResultUnderCursorbyChannel (Variables|Default|GetPlayerController) "TraceTypeQuery4" true)))))) (Transformation|GetActorLocation (.HitActor (Collision|BreakHitResult (.HitResult (Game|Player|GetHitResultUnderCursorbyChannel (Variables|Default|GetPlayerController) "TraceTypeQuery4" true))))) (.Location (Collision|BreakHitResult (.HitResult (Game|Player|GetHitResultUnderCursorbyChannel (Variables|Default|GetPlayerController) "TraceTypeQuery4" true))))))))))
                (:then_1
                  (Transformation|SetActorLocation (Variables|Default|GetRainOfArrowsTarget) (.Location (Collision|BreakHitResult (.HitResult (Game|Player|GetHitResultUnderCursorbyChannel (Variables|Default|GetPlayerController) "TraceTypeQuery4" true)))) false true))))))))
    (else
      (Ability|CancelAbility))))

(event Ability|EventOnEndAbility
  (params (bWasCancelled :type Boolean))
  (if bWasCancelled
    (Actor|DestroyActor (Variables|Default|GetRainOfArrowsTarget))))
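; Gameplay ability for the Archer's dash, moving the player along the last movement input or facing direction.
; After committing, the authority applies additive constant-force root motion with clamped exit velocity, broadcasts the cooldown and snaps rotation to the dash unless aiming.
; When root motion finishes, a delay holds the ability open to prevent immediate action cancelling.
; Directional montage selection and playback logic exists but is disconnected from activation.
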(event Ability|EventActivateAbility
  (bind _returnvalue (Ability|GetAvatarActorfromActorInfo))
  (bind (_facing _last_movement_input _positive) (|GetDirection_2))
  ;[0.01042 0.01042 0.01042] Calculate dash direction and select appropriate animation
  (bind _output_get (Variables|Dash|SetDirection (select _positive _last_movement_input _facing)))
  ;[0.01042 0.01042 0.01042] If we have a non-zero dash, commit the ability
  (if (Math|Vector|VectorIsNearlyZero _output_get)
    (Ability|CancelAbility :!label _label)
    (else
      (bind _returnvalue_2 (Ability|CommitAbility))
      (if _returnvalue_2
        (Ability|HasAuthority
          (:True
            (Utilities|FlowControl|Sequence
              (:then_0
                ;[0.01042 0.01042 0.01042] Use values to apply root motion to pawn
                (Ability|Tasks|ApplyRootMotionConstantForce "None" (Variables|Dash|GetDirection) (Variables|Dash|GetStrength) (Variables|Dash|GetRootMotionDuration) true 0 "ClampVelocity" (Transformation|GetVelocity _returnvalue) 1e+03
                  (:OnFinish
                    ;[0.01042 0.01042 0.01042] Delay end of ability so you can't immediately cancel into another action
                    (Utilities|FlowControl|Delay (- (Variables|Dash|GetAbilityDuration) (Variables|Dash|GetRootMotionDuration)))
                    (Ability|EndAbility))))
              (:then_1
                (CallFunction|BroadcastCooldown) ; Update UI
              )
              (:then_2
                ;[0.01042 0.01042 0.01042] If we are not aiming
                (bind _returnvalue_3 (Class|ArcherPlayerCharacter|GetIsAiming (Class|ArcherGameplayAbility|GetArcherPlayerCharacterfromActorInfo)))
                (if (not _returnvalue_3)
                  ;[0.01042 0.01042 0.01042] Rotate towards dashing direction
                  (Transformation|SetActorRotation _returnvalue (Math|Conversions|RotationFromXVector (Variables|Dash|GetDirection)) true))))))
        (else
          (goto _label))))))

(fn CalculateAnimPlayRate
  (return (/ (/ (Animation|GetPlayLength (Variables|Dash|Montage|GetMontage)) (Variables|Dash|GetRootMotionDuration)) 4.0)))

(fn SelectDirectionalMontage
  (params (FacingDirection :type Vector) (MovementDirection :type Vector))
  (bind _returnvalue (Class|DirectionalAnimationDataAsset|GetMontagefromDeltaAngle (Variables|Default|GetDashDirectionalMontageAsset) (.yaw (Math|Rotator|MakeRotfromX (select (Utilities|Operators|NotEqual(!=) :A MovementDirection) MovementDirection FacingDirection)))))
  (return _returnvalue))
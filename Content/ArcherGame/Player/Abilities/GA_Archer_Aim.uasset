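; Archer aim Gameplay Ability that charges shot power while the aim input is held.
; A tick task turns control yaw toward the cursor and, unless the Event.Shooting tag is present, shows and fills the power slider.
; On release it writes the power into the GA_Archer_Shoot instance, activates it and ends.
; It also sizes the slider from a pooled arrow's max speed and temporarily overrides character rotation rate.
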(event Ability|EventActivateAbility
  (bind _returnvalue (Class|ArcherGameplayAbility|GetArcherPlayerCharacterfromActorInfo))
  (bind _returnvalue_2 (Class|ArcherGameplayAbility|GetArcherPlayerCharacterfromActorInfo))
  (bind _returnvalue_3 (Class|ArcherPlayerCharacter|GetPlayerController _returnvalue_2))
  (bind _charactermovement (Variables|/Script/Engine.Character|GetCharacterMovement _returnvalue))
  (bind _returnvalue_4 (Ability|CommitAbility))
  (if _returnvalue_4
    (Utilities|FlowControl|Sequence
      (:then_0
        (CallFunction|GetAbilitySystemNShootAbility))
      (:then_1
        (CallFunction|SetShootingPowerWidgetSize))
      (:then_2
        ;[1 1 1] If player releases aim button, try playing shooting ability and end ability
        (Ability|Tasks|WaitInputRelease false
          (:OnRelease
            (Variables|/Game/ArcherGame/Player/Abilities/Shooting/GA_Archer_Shoot.GA_Archer_Shoot_C|SetShootingPower (Variables|Ability|Shoot|GetShootAbility) (Variables|ShootingPower|GetShootingPower))
            (Class|AbilitySystemComponent|TryActivateAbility (Variables|Ability|GetArcherAbilitySystemComponent) (Variables|Ability|Shoot|GetShootGameplayAbilitySpecHandle) true)
            (Ability|EndAbility))))
      (:then_3
        ;[1 1 1] Set power increase speed
        (Variables|ShootingPower|SetShootingPowerIncreaseSpeed (/ 1.0 (Variables|ShootingPower|GetFullShootingPowerTime)))
        (Variables|ShootingPower|SetShootingPower (Variables|ShootingPower|GetMinShootingPower)))
      (:then_4
        (bind _deltatime (|AbilityTaskonTick "None")
          (:OnTickTaskDelegate
            (Utilities|FlowControl|Sequence
              (:then_0
                ;[1 1 1] Handle shooting power widget visibility
                (bind _output_get (Variables|Ability|Shoot|SetCanShoot (not (GameplayTags|HasMatchingGameplayTag (Variables|Ability|GetArcherAbilitySystemComponent) "(TagName=\"Event.Shooting\")"))))
                (Widget|SetVisibility (Variables|Widget|GetShootPowerWidget) (select _output_get "Visible" "Hidden")))
              (:then_1
                ;[1 1 1] Set actor control rotation
                (Pawn|SetControlRotation _returnvalue_3 (Math|Rotator|MakeRotator 0.0 0.0 (.yaw (Math|Rotator|FindLookatRotation (Class|PlayerController|GetFocalLocation _returnvalue_3) (.Location (Collision|BreakHitResult (.HitResult (Game|Player|GetHitResultUnderCursorbyChannel _returnvalue_3 "TraceTypeQuery3" true)))))))))
              (:then_2
                ;[1 1 1] increase power untill its <= 1
                (if (and (<= (Variables|ShootingPower|GetShootingPower) 1.0) (Variables|Ability|Shoot|GetCanShoot))
                  (bind _output_get_2 (Variables|ShootingPower|SetShootingPower (+ (Variables|ShootingPower|GetShootingPower) (* _deltatime (Variables|ShootingPower|GetShootingPowerIncreaseSpeed)))))
                  ;[1 1 1] Set shooting power widget percent
                  (Variables|/Game/ArcherGame/Player/Shooting/Widget/WBP_ShootPowerSlider.WBP_ShootPowerSlider_C|SetPercent (Variables|Widget|GetShootPowerWidget) _output_get_2)))))))
      (:then_5
        ;[1 1 1] Set character movement rotation rate to something faster and save the old one
        (Variables|RotationRate|SetOldRotationRate (Variables|/Script/Engine.CharacterMovementComponent|GetRotationRate _charactermovement))
        (Variables|/Script/Engine.CharacterMovementComponent|SetRotationRate _charactermovement (Variables|RotationRate|GetAimingRotationRate))))))

(event Ability|EventOnEndAbility
  (params (bWasCancelled :type Boolean))
  ;[1 1 1] Set old rotation rate back to character movement
  (Variables|/Script/Engine.CharacterMovementComponent|SetRotationRate (Variables|/Script/Engine.Character|GetCharacterMovement (Class|ArcherGameplayAbility|GetArcherPlayerCharacterfromActorInfo)) (Variables|RotationRate|GetOldRotationRate))
  ;[1 1 1] Hide shooting power widget
  (Widget|SetVisibility (Variables|Widget|GetShootPowerWidget) "Hidden"))

(fn SetShootingPowerWidgetSize
  ;[1 1 1] find arrow projectile from arrow pooler's pooled actors and get its projectile component max speed for widget
  (bind _returnvalue (Class|PoolerBlueprintFunctionLibrary|GetPoolerbyGameplayTag "(TagName=\"Pool.Arrow\")"))
  (bind _asarrow_projectile (Utilities|Casting|CastToArrowProjectile (Components|GetOwner (Utilities|Array|Get(acopy) (Variables|/Script/Pooling.Pooler|GetPooledActors _returnvalue)))))
  ;[1 1 1] Get player blueprint for widget
  (bind _asbp_player (Utilities|Casting|CastToBP_Player (Class|ArcherGameplayAbility|GetArcherPlayerCharacterfromActorInfo)))
  ;[1 1 1] Set shoot power slider offset
  (Variables|Widget|SetShootPowerWidget (Variables|/Game/ArcherGame/Player/BP_Player.BP_Player_C|GetShootPowerSlider _asbp_player))
  (Class|CanvasPanelSlot|SetOffsets (Class|WidgetLayoutLibrary|SlotasCanvasSlot (Variables|/Game/ArcherGame/Player/Shooting/Widget/WBP_ShootPowerSlider.WBP_ShootPowerSlider_C|GetSizeBox (Variables|Widget|GetShootPowerWidget))) (Utilities|Struct|MakeMargin (* (Variables|/Script/Engine.ProjectileMovementComponent|GetMaxSpeed (Variables|/Script/ArcherGame.ArcherProjectileBase|GetProjectileMovementComponent _asarrow_projectile)) 0.35) (.top (Class|CanvasPanelSlot|GetOffsets (Class|WidgetLayoutLibrary|SlotasCanvasSlot (Variables|/Game/ArcherGame/Player/Shooting/Widget/WBP_ShootPowerSlider.WBP_ShootPowerSlider_C|GetSizeBox (Variables|Widget|GetShootPowerWidget))))) (.right (Class|CanvasPanelSlot|GetOffsets (Class|WidgetLayoutLibrary|SlotasCanvasSlot (Variables|/Game/ArcherGame/Player/Shooting/Widget/WBP_ShootPowerSlider.WBP_ShootPowerSlider_C|GetSizeBox (Variables|Widget|GetShootPowerWidget))))) (.bottom (Class|CanvasPanelSlot|GetOffsets (Class|WidgetLayoutLibrary|SlotasCanvasSlot (Variables|/Game/ArcherGame/Player/Shooting/Widget/WBP_ShootPowerSlider.WBP_ShootPowerSlider_C|GetSizeBox (Variables|Widget|GetShootPowerWidget))))))))

(fn GetAbilitySystemNShootAbility
  (bind _returnvalue (Class|ArcherGameplayAbility|GetArcherPlayerCharacterfromActorInfo))
  (bind _returnvalue_2 (Class|ArcherCharacter|GetArcherAbilitySystemComponent _returnvalue))
  (Variables|Ability|SetArcherAbilitySystemComponent _returnvalue_2)
  (bind _out_gameplayabilityspechandle (Class|ArcherAbilitySystemComponent|FindAbilitySpecHandlefromTag _returnvalue_2 "(TagName=\"Ability.Shooting\")"))
  (bind _output_get (Variables|Ability|Shoot|SetShootGameplayAbilitySpecHandle _out_gameplayabilityspechandle))
  (bind _asga_archer_shoot (Utilities|Casting|CastToGA_Archer_Shoot (.ReturnValue (Ability|GameplayAbility|GetGameplayAbilityfromSpecHandle (Variables|Ability|GetArcherAbilitySystemComponent) _output_get))))
  (Variables|Ability|Shoot|SetShootAbility _asga_archer_shoot))
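; Actor that displays a floating damage number at a given location through a WBP_FloatingNumber on its widget component.
; PlayFloatingNumber sets the widget's damage amount and teleports the actor to the play location.
; The widget reference is lazily cast and cached on first access.
; BeginPlay binds to the end of the pop animation, which destroys the actor rather than pooling it as an inline comment suggests.
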(event Custom|OnAnimationFinished
  ;[1 1 1] Bind to animation end event and return to pool when it ended
  (Actor|DestroyActor))

(event EventBeginPlay
  (bind _floatingnumberwidget (CallFunction|GetFloatingNumberWidget))
  ;[1 1 1] Bind to animation end event and return to pool when it ended
  (Class|UserWidget|BindtoAnimationEvent _floatingnumberwidget (Variables|/Game/ArcherGame/Effects/FloatingDamageNumbers/WBP_FloatingNumber.WBP_FloatingNumber_C|GetPopFloatingNumber _floatingnumberwidget) (delegate Custom|OnAnimationFinished) "Finished" "None"))

(event Collision|EventActorBeginOverlap
  (params (OtherActor :type Actor%20Object%20Reference)))

(event EventTick
  (params (DeltaSeconds :type Float%20%28single-precision%29)))

(fn ConstructionScript)

(fn PlayFloatingNumber
  (params (DamageAmount :type Float%20%28double-precision%29) (PlayLocation :type Vector))
  (bind _floatingnumberwidget (CallFunction|GetFloatingNumberWidget))
  (Variables|/Game/ArcherGame/Effects/FloatingDamageNumbers/WBP_FloatingNumber.WBP_FloatingNumber_C|SetDamageAmount _floatingnumberwidget DamageAmount)
  (Transformation|SetActorLocation PlayLocation false true))

(fn GetFloatingNumberWidget
  (if (Utilities|IsValid (Variables|Default|GetFloatingNumberWidget))
    _
    (else
      (bind _aswbp_floating_number (Utilities|Casting|CastToWBP_FloatingNumber (UserInterface|GetUserWidgetObject (Variables|Default|GetWidget))))
      (Variables|Default|SetFloatingNumberWidget _aswbp_floating_number)))
  (return (Variables|Default|GetFloatingNumberWidget)))